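; Inventory component that creates an inventory widget on BeginPlay and toggles it on screen with the I key.
; E runs a sphere trace around the player's lower body to find a BP_item.
; The hit item's quantity merges into same-name entries in the item array if it is stackable and the total stays within the stack cap.
; The graph neither adds new entries nor removes the picked-up actor.
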(event `self.ReceiveBeginPlay`
  (bind _returnvalue (`|CreateWidget` "/Game/runner/Blueprints/inventory/Widget/WB_inventory.WB_inventory_C"))
  (set `self.InventoryWidget` _returnvalue))

(event `Key|I`
  (params (Key :type "Key Structure"))
  (bind _inventorywidget (`self.InventoryWidget`))
  (:`Pressed`
    (if (`Widget.IsVisible` (`self.InventoryWidget`))
      (`Widget.RemoveFromParent` _inventorywidget)
      (else
        (`UserWidget.AddToViewport` _inventorywidget 0)))))

(event `Key|E`
  (params (Key :type "Key Structure"))
  (bind _returnvalue (- (`Actor.K2_GetActorLocation` (`GameplayStatics.GetPlayerCharacter` 0)) (0.0 0.0 65.0)))
  (:`Pressed`
    (bind _outhit (`KismetSystemLibrary.SphereTraceSingle` _returnvalue _returnvalue 120.0 "TraceTypeQuery1"))
    (bind _asbp_item (cast `/Game/runner/Blueprints/inventory/Blueprints2/BP_item` (`.HitActor` (`GameplayStatics.BreakHitResult` _outhit))))
    (for (_array_element _array_index) (`|MakeArray` (`self.Item`))
      (bind (_name _stackable _quantity) (break `/Game/runner/Blueprints/inventory/Blueprints2/S_itemStruct` _array_element))
      (bind (_name_2 _stackable_2 _quantity_2) (break `/Game/runner/Blueprints/inventory/Blueprints2/S_itemStruct` (`/Game/runner/Blueprints/inventory/Blueprints2/BP_item.item` _asbp_item)))
      (bind _returnvalue_2 (+ _quantity _quantity_2))
      (if (and (`KismetTextLibrary.EqualEqual_TextText` _name _name_2) _stackable_2 (<= _returnvalue_2 64))
        (bind (_item_name _item_stackable _item_quantity _item_thumnail _item_mesh) (break `/Game/runner/Blueprints/inventory/Blueprints2/S_itemStruct` (`/Game/runner/Blueprints/inventory/Blueprints2/BP_item.item` _asbp_item)))
        (`KismetArrayLibrary.Array_Set` (`|MakeArray` (`self.Item`)) _array_index (make `/Game/runner/Blueprints/inventory/Blueprints2/S_itemStruct` _item_name _item_stackable _returnvalue_2 _item_thumnail _item_mesh))))))